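; BP_Target is a shootable, timed target that drives score and timer changes in the shooter game mode.
; BeginPlay sets its lifespan and a matching delay, after which it adjusts TargetHolder and deducts score.
; A BP_ShooterProjectile_Bullet hit on the cylinder runs the same holder adjustment, adds score and timer time, then destroys the target shortly after.
; That shared adjustment recalculates TargetHolder's NewLifeSpan and SpawnTimer using Value.
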(event `self.ReceiveBeginPlay`
  (bind _value (`self.value`))
  (bind _lifespan (`self.LIfeSpan`))
  (bind _targetholder (`self.TargetHolder`))
  (`self.SetLifeSpan` _lifespan)
  (`KismetSystemLibrary.Delay` _lifespan)
  (`|ExecutionSequence`
    (:`then_0`
      (set `/Game/Blueprints/BP_TargetHolder.NewLifeSpan` (/ (`/Game/Blueprints/BP_TargetHolder.NewLifeSpan` _targetholder) _value) _targetholder :!label _label)
      (set `/Game/Blueprints/BP_TargetHolder.SpawnTimer` (/ _value (`/Game/Blueprints/BP_TargetHolder.SpawnTimer` _targetholder)) _targetholder))
    (:`then_1`
      (bind _asbp_shooter_game_mode (cast `/Game/Variant_Shooter/Blueprints/BP_ShooterGameMode` (`GameplayStatics.GetGameMode`)))
      (`ShooterGameMode.IncrementScore` _asbp_shooter_game_mode -11))))

(event `self.Cylinder.OnComponentHit`
  (params (HitComponent :type "PrimitiveComponent Object Reference") (OtherActor :type "Actor Object Reference") (OtherComp :type "PrimitiveComponent Object Reference") (NormalImpulse :type "Vector Structure") (Hit :type "HitResult Structure (by ref)"))
  (if (== (`GameplayStatics.GetObjectClass` OtherActor) "/Game/Variant_Shooter/Blueprints/Pickups/Projectiles/BP_ShooterProjectile_Bullet.BP_ShooterProjectile_Bullet_C")
    (`|ExecutionSequence`
      (:`then_0`
        (goto _label))
      (:`then_1`
        (bind _asbp_shooter_game_mode (cast `/Game/Variant_Shooter/Blueprints/BP_ShooterGameMode` (`GameplayStatics.GetGameMode`)))
        (`ShooterGameMode.IncrementScore` _asbp_shooter_game_mode 13)
        (`ShooterGameMode.IncrementTimer` _asbp_shooter_game_mode 0.35)
        (`KismetSystemLibrary.Delay` 0.1)
        (`self.K2_DestroyActor`)))))

(fn `UserConstructionScript`)