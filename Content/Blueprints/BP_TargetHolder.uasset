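; BP_TargetHolder spawns BP_Target actors at random points within the bounds of its SpawnArea component.
; From BeginPlay, a looping sequence picks a point, then waits SpawnTimer before spawning there and incrementing NumberOfTargets.
; The loop re-enters above the counter reset, so NumberOfTargets returns to zero before each MaxTargets check and spawning continues indefinitely whenever MaxTargets is non-negative.
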(event `self.ReceiveBeginPlay`
  (bind (_origin _boxextent) (`KismetSystemLibrary.GetComponentBounds` (`self.SpawnArea`)))
  (`|ExecutionSequence` :!label _label
    (:`then_0`
      (set `self.RandomPoint` (`KismetMathLibrary.RandomPointInBoundingBox` _origin _boxextent))
      (set `self.NumberOfTargets` 0))
    (:`then_1`
      (if (>= (`self.MaxTargets`) (`self.NumberOfTargets`))
        (`KismetSystemLibrary.Delay` (`self.SpawnTimer`))
        (`|SpawnActorFromClass` "/Game/Blueprints/BP_Target.BP_Target_C" (`KismetMathLibrary.MakeTransform` (`self.RandomPoint`)) "Undefined" "MultiplyWithRoot" null null)
        (set `self.NumberOfTargets` (+ 1 (`self.NumberOfTargets`)))
        (goto _label)
        (else
          (`KismetSystemLibrary.PrintString` "Max targets reached"))))))

(fn `UserConstructionScript`)